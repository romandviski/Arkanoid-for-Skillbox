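; BP_Block_Castle is an Arkanoid block variant featuring a treasure chest that pops open when hit.
; On Hit, it rotates the chest lid to a fixed open angle, spawns a coin-burst Niagara effect at its location, then forwards the hit to the parent block logic.
; The open effect runs on every hit, as the LifeComponent alive check is left unconnected.
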(event EventBeginPlay
  (|CallParentFunction))

(event Collision|EventActorBeginOverlap
  (params (OtherActor :type Actor%20Object%20Reference))
  (|CallParentFunction OtherActor) ; This node is disabled and will not be called.\nDrag off pins to build functionality.
)

(event EventTick
  (params (DeltaSeconds :type Float%20%28single-precision%29))
  (|CallParentFunction DeltaSeconds) ; This node is disabled and will not be called.\nDrag off pins to build functionality.
)

(event Collision|EventHit
  (params (MyComp :type Primitive%20Component%20Object%20Reference) (Other :type Actor%20Object%20Reference) (OtherComp :type Primitive%20Component%20Object%20Reference) (bSelfMoved :type Boolean) (HitLocation :type Vector :default "0, 0, 0") (HitNormal :type Vector :default "0, 0, 0") (NormalImpulse :type Vector :default "0, 0, 0") (Hit :type Hit%20Result%20Structure%20%28by%20ref%29))
  (Utilities|FlowControl|Sequence
    (:then_0
      (Transformation|SetRelativeRotation (Variables|Default|GetSM_Prop_Chest_03_Lid) "0.000000,0.000000,-95.000000" false false)
      (Niagara|SpawnSystematLocation "/Game/CharacterBodyFX/FX/Coins/NS_BlowCoins.NS_BlowCoins" (Transformation|GetActorLocation)))
    (:then_1
      (|CallParentFunction MyComp Other OtherComp bSelfMoved HitLocation HitNormal NormalImpulse Hit))))

(fn ConstructionScript
  (|CallParentFunction))